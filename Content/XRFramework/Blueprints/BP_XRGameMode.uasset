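; XR game mode for the archery game, handling score, player naming and leaderboard loading.
; On BeginPlay it caches the archery Game Instance, then loads the save's leaderboard into it or creates a new save.
; StartGame builds a random player name from Alphabet entries, and AddScore keeps a printed running total.
; FinishGame is unfinished: it only adds an empty name to the current difficulty's leaderboard entry, without score or saving.
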(event EventBeginPlay
  (bind _asgi_archery_game (Utilities|Casting|CastToGI_ArcheryGame (Game|GetGameInstance)))
  (Variables|Default|SetAs%20GI%20Archery%20Game _asgi_archery_game)
  (CallFunction|LoadGame))

(fn ConstructionScript)

(fn AddScore
  (params (ScoreToAdd :type Integer))
  (bind _output_get (Variables|Default|SetCurrentScore (+ (Variables|Default|GetCurrentScore) ScoreToAdd)))
  (Development|PrintString (Utilities|String|Append "Total Score : " (Utilities|String|ToString(Integer) _output_get)) true true "(R=0.046578,G=1.000000,B=0.000000,A=1.000000)"))

(fn FinishGame
  (bind _as_gi_archery_game (Variables|Default|GetAs%20GI%20Archery%20Game)
    (:then
      (Utilities|Array|Add (.PlayerName (Utilities|Struct|BreakS_LeaderBoard (.Value (Utilities|Map|Find (Variables|/Game/ArcheryGame/Blueprints/Core/GI_ArcheryGame.GI_ArcheryGame_C|GetLeaderBoard _as_gi_archery_game) (Variables|Default|GetCurrentDifficulty))))) ""))
    (:else)))

(fn LoadGame
  (bind _returnvalue (SaveGame|DoesSaveGameExist (Variables|Default|GetSaveGameName)))
  (if _returnvalue
    (bind _returnvalue_2 (SaveGame|LoadGamefromSlot (Variables|Default|GetSaveGameName)))
    (bind _assg_archery (Utilities|Casting|CastToSG_Archery _returnvalue_2))
    (bind _output_get (Variables|Default|SetSaveGameObject _assg_archery))
    (Variables|/Game/ArcheryGame/Blueprints/Core/GI_ArcheryGame.GI_ArcheryGame_C|SetLeaderBoard (Variables|Default|GetAs%20GI%20Archery%20Game) (Variables|/Game/ArcheryGame/Blueprints/Core/SG_Archery.SG_Archery_C|GetLeaderBoard _output_get))
    (Development|PrintString "SAVE GAME LOADED" true true "(R=0.000000,G=0.184445,B=1.000000,A=1.000000)")
    (else
      (bind _returnvalue_3 (SaveGame|CreateSaveGameObject "/Game/ArcheryGame/Blueprints/Core/SG_Archery.SG_Archery_C"))
      (bind _output_get_2 (Variables|Default|SetSaveGameObject _returnvalue_3))
      (SaveGame|SaveGametoSlot _output_get_2 (Variables|Default|GetSaveGameName))
      (Development|PrintString "SAVE GAME CREATED" true true "(R=1.000000,G=0.464789,B=0.000000,A=1.000000)"))))

(fn StartGame
  (PlayerName|CreateRNDName))

(fn CreateRNDName
  (bind _playernamearray (LocalVariables|GetPlayerNameArray))
  (for _index (range 0 2)
    (if (Utilities|Array|IsValidIndex _playernamearray _index)
      (Utilities|Array|SetArrayElem (LocalVariables|GetPlayerNameArray) _index (.OutItem (Utilities|Array|Random (Variables|Hidden|GetAlphabet))))))
  (Variables|Default|SetPlayerName (PlayerName|MakeName _playernamearray)))

(fn MakeName
  (params (Array :type Array%20of%20Strings))
  (LocalVariables|SetNewName "")
  (for _array_element Array
    (LocalVariables|SetNewName (Utilities|String|Append (LocalVariables|GetNewName) _array_element)))
  (return (LocalVariables|GetNewName)))