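; BP_GrabManager is a component on BP_XRPawn that clears one hand's held-component reference when a grabbed component is released.
; On BeginPlay it casts its owner to the pawn and caches it, printing a failure message otherwise.
; BindEventReleased hooks a grab component's release event to Release, which nulls the pawn's right or left held component based on the IsRightHandManager flag.
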(event Custom|BindEventReleased
  (params (GrabComponent :type BP%20Grab%20Component%20Object%20Reference%20%28by%20ref%29))
  (Utilities|IsValid GrabComponent
    (:Is%20Valid
      (EventDispatchers|BindEventtoOnComponentReleased GrabComponent (delegate Custom|Release)))))

(event Custom|Release
  (bind _as_bp_xrpawn (Variables|Default|GetAs%20BP%20XRPawn))
  (Variables|Default|GetAs%20BP%20XRPawn
    (:then
      (if (Variables|Default|GetisRightHandManager)
        (Variables|/Game/ArcheryGame/Blueprints/Core/BP_XRPawn.BP_XRPawn_C|SetHeldComponentRight _as_bp_xrpawn 0)
        (else
          (Variables|/Game/ArcheryGame/Blueprints/Core/BP_XRPawn.BP_XRPawn_C|SetHeldComponentLeft _as_bp_xrpawn 0))))
    (:else)))

(event EventBeginPlay
  (bind _asbp_xrpawn (Utilities|Casting|CastToBP_XRPawn (Components|GetOwner))
    (:then
      (Variables|Default|SetAs%20BP%20XRPawn _asbp_xrpawn))
    (:CastFailed
      (Development|PrintString "FAIL" true true "(R=1.000000,G=0.014121,B=0.000000,A=1.000000)" 15.0))))