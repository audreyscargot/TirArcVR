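; Game instance Blueprint for the archery game that re-sorts the per-level leaderboards and then saves.
; UpdateLeaderBoard runs MakeLeaderBoard on each map entry, then calls SaveGame on BP_XRGameMode.
; MakeLeaderBoard repeatedly moves the highest score and its name from working arrays into new ones, ordering scores descending.
; Only the name array is reversed before both are written back to the map, so names end opposite to their scores.
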(fn UpdateLeaderBoard
  (bind _leaderboardlevel (Variables|Default|GetLeaderBoardLevel))
  (bind (_keypin _valuepin) (Utilities|Map|ForEachLoop(Map) _leaderboardlevel)
    (:then
      (CallFunction|MakeLeaderBoard _leaderboardlevel _valuepin _keypin))
    (:CompletedPin
      (bind _asbp_xrgame_mode (Utilities|Casting|CastToBP_XRGameMode (Game|GetGameMode)))
      (Default|SaveGame _asbp_xrgame_mode))))

(fn MakeLeaderBoard
  (params (TargetMap :type Map%20of%20Integers%20to%20Structs) (S_LeaderBoard :type S%20Leader%20Board%20Structure%20%28by%20ref%29) (Level :type Integer%20%28by%20ref%29))
  (bind _value (Utilities|Map|Find TargetMap Level))
  (bind _cleararrayname (LocalVariables|GetClearArrayName))
  (bind (_playername _score) (Utilities|Struct|BreakS_LeaderBoard _value))
  (LocalVariables|SetTempArryName _playername)
  (LocalVariables|SetTempArray _score)
  (while (> (Utilities|Array|Length (LocalVariables|GetTempArray)) 0)
    (Utilities|Array|Add (LocalVariables|GetClearArray) (.MaxValue (Math|Integer|MaxOfIntArray (LocalVariables|GetTempArray))))
    (Utilities|Array|Add (LocalVariables|GetClearArrayName) (Utilities|Array|Get(acopy) (LocalVariables|GetTempArryName) (.IndexOfMaxValue (Math|Integer|MaxOfIntArray (LocalVariables|GetTempArray)))))
    (Utilities|Array|RemoveIndex (LocalVariables|GetTempArryName) (.IndexOfMaxValue (Math|Integer|MaxOfIntArray (LocalVariables|GetTempArray))))
    (Utilities|Array|RemoveIndex (LocalVariables|GetTempArray) (.IndexOfMaxValue (Math|Integer|MaxOfIntArray (LocalVariables|GetTempArray)))))
  (Utilities|Array|Reverse _cleararrayname)
  (Utilities|Map|Add TargetMap Level (Utilities|Struct|MakeS_LeaderBoard _cleararrayname (LocalVariables|GetClearArray))))