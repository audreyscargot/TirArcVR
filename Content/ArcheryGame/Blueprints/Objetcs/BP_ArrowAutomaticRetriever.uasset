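; BP_ArrowAutomaticRetriever is a trigger volume that returns arrows entering it to the arrow spawner.
; On BeginPlay it caches the BP_ArrowSpawner found in the level.
; When a BP_Arrow overlaps its Box, it turns off the grab component's physics, moves the arrow to the spawner's location with the ArrowIndicator's rotation, then re-enables physics after a short delay.
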(event OnComponentBeginOverlap(Box)
  (params (OverlappedComponent :type Primitive%20Component%20Object%20Reference) (OtherActor :type Actor%20Object%20Reference) (OtherComp :type Primitive%20Component%20Object%20Reference) (OtherBodyIndex :type Integer) (bFromSweep :type Boolean) (SweepResult :type Hit%20Result%20Structure%20%28by%20ref%29))
  (bind _spawnerref (Variables|Default|GetSpawnerRef))
  (bind _asbp_arrow (Utilities|Casting|CastToBP_Arrow OtherActor))
  (Utilities|IsValid _spawnerref
    (:Is%20Valid
      (Default|SetPrimitiveCompPhysics (Variables|/Game/ArcheryGame/Blueprints/Parents/BP_Grabbable.BP_Grabbable_C|GetBP_GrabComponent _asbp_arrow) false)
      (Transformation|SetActorLocationAndRotation _asbp_arrow (Transformation|GetActorLocation _spawnerref) (Transformation|GetWorldRotation (Variables|/Game/ArcheryGame/Blueprints/Objetcs/BP_ArrowSpawner.BP_ArrowSpawner_C|GetArrowIndicator _spawnerref)))
      (Utilities|FlowControl|Delay 0.2)
      (Default|SetPrimitiveCompPhysics (Variables|/Game/ArcheryGame/Blueprints/Parents/BP_Grabbable.BP_Grabbable_C|GetBP_GrabComponent _asbp_arrow) true))))

(event EventBeginPlay
  (bind _returnvalue (Actor|GetActorOfClass "/Game/ArcheryGame/Blueprints/Objetcs/BP_ArrowSpawner.BP_ArrowSpawner_C"))
  (Variables|Default|SetSpawnerRef _returnvalue))

(fn ConstructionScript)