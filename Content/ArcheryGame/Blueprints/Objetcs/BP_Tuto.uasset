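; BP_Tuto is an animated marker in the archery game, apparently a tutorial arrow, that moves and blinks to draw attention.
; On BeginPlay it caches its world location and plays the Movement timeline, whose ArrowMov track, scaled by Time, drives a vertical Lerp offset on the root.
; The timeline update also enters a self-looping Delay chain that swaps the Plane's material between red and normal variants every half second.
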(event EventBeginPlay
  (bind _plane (Variables|Default|GetPlane))
  (Variables|Default|SetStart%20Location (Transformation|GetWorldLocation (Variables|Default|GetDefaultSceneRoot)))
  (bind _arrowmov (Timeline|Movement Play)
    (:Update
      (Transformation|SetRelativeLocation (Variables|Default|GetDefaultSceneRoot) (+ (Math|Vector|MakeVector 0.0 0.0 (Math|Float|Lerp 0.0 -5.0 (* _arrowmov (Variables|Default|GetTime)))) (Variables|Default|GetStart%20Location)) false false)
      (Rendering|Material|SetMaterial _plane 0 "/Game/ArcheryGame/Blueprints/Objetcs/IDGAFLF_butred.IDGAFLF_butred" :!label _label)
      (Utilities|FlowControl|Delay 0.5)
      (Rendering|Material|SetMaterial _plane 0 "/Game/ArcheryGame/Blueprints/Objetcs/IDGAFLF.IDGAFLF")
      (Utilities|FlowControl|Delay 0.5)
      (goto _label))))

(fn ConstructionScript)