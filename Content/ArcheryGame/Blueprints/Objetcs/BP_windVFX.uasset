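; Wind effect actor for the archery game that spawns Niagara wind visuals matching each level's wind.
; It binds to the XR game mode's PreparingTarget event, picks a wind direction from the level index and starts four looping timers with randomized intervals.
; The spawn event places NS_Wind at a random point within a scaled box, passing in direction and a multiple of WindStrength before activating it.
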(event Custom|MakeWindref
  (params (IntegerLevelDifficulty :type E_Difficulty%20Enum :default "NewEnumerator0") (IntegerLevel :type Integer))
  (Variables|Default|SetWindDirection (Utilities|Select :Index IntegerLevel :Option%200 "0.000000,0.000000,0.000000" :Option%201 "0, 0, 0" :Option%202 "0.000000,-1.000000,0.000000" :Option%203 "0, 0, 0" :Option%204 "1.000000,1.000000,0.000000" :Option%205 "1.000000,0.000000,0.000000" :Option%206 "1.000000,-1.000000,0.000000" :Option%207 "-1.000000,-1.000000,0.000000" :Option%208 "-1.000000,0.000000,0.000000"))
  (Utilities|Time|SetTimerbyEvent (EventDispatchers|CreateEvent :!event Custom|spawnVFX) (Math|Random|RandomFloatinRange (Variables|Default|GetMin) (Variables|Default|GetMax)) true)
  (Utilities|Time|SetTimerbyEvent (EventDispatchers|CreateEvent :!event Custom|spawnVFX) (Math|Random|RandomFloatinRange (Variables|Default|GetMin) (Variables|Default|GetMax)) true)
  (Utilities|Time|SetTimerbyEvent (EventDispatchers|CreateEvent :!event Custom|spawnVFX) (Math|Random|RandomFloatinRange (Variables|Default|GetMin) (Variables|Default|GetMax)) true)
  (Utilities|Time|SetTimerbyEvent (EventDispatchers|CreateEvent :!event Custom|spawnVFX) (Math|Random|RandomFloatinRange (Variables|Default|GetMin) (Variables|Default|GetMax)) true))

(event Custom|spawnVFX
  (bind _box (Variables|Default|GetBox))
  (bind _returnvalue (Transformation|GetWorldScale _box))
  (bind _returnvalue_2 (Niagara|SpawnSystematLocation "/Game/XRFramework/VFX/NS_Wind.NS_Wind" (Math|Random|RandomPointinBoundingBox (Transformation|GetWorldLocation (Variables|Default|GetBox)) (Math|Vector|MakeVector (* (.x _returnvalue) 3e+01) (* (.y _returnvalue) 3e+01) (* (.z _returnvalue) 3e+01))) "0, 0, 0" "1.000000,1.000000,1.000000" true false))
  (Class|NiagaraComponent|SetNiagaraVariableVec3 _returnvalue_2 "WindDirection" (Variables|Default|GetWindDirection))
  (Niagara|SetNiagaraVariable(Float) _returnvalue_2 "WindSpeed" (* (Variables|Default|GetWindStrength) 3.0))
  (Components|Activation|Activate _returnvalue_2 false))

(event EventBeginPlay
  (bind _asbp_xrgame_mode (Utilities|Casting|CastToBP_XRGameMode (Game|GetGameMode)))
  (EventDispatchers|BindEventtoPreparingTarget _asbp_xrgame_mode (delegate Custom|MakeWindref)))

(fn ConstructionScript)