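; VR bow actor that nocks a grabbed arrow and fires it when the draw grip is dropped.
; A box overlap takes one arrow from the hand, snaps it to a left- or right-handed spot, attaches it and enables the grab components.
; Dropping the draw grip detaches the arrow and calls the XR pawn's Shoot along the bow's forward vector.
; Tick draws a debug grab sphere; arrow-pull logic is an unconnected experiment.
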(event OnComponentBeginOverlap(Box)
  (params (OverlappedComponent :type Primitive%20Component%20Object%20Reference) (OtherActor :type Actor%20Object%20Reference) (OtherComp :type Primitive%20Component%20Object%20Reference) (OtherBodyIndex :type Integer) (bFromSweep :type Boolean) (SweepResult :type Hit%20Result%20Structure%20%28by%20ref%29))
  (bind (_locationvalue _rotatorvalue) (CallFunction|GetArrowLocation))
  (bind _asbp_arrow (Utilities|Casting|CastToBP_Arrow OtherActor))
  (Variables|Default|GetAs%20BP%20Arrow
    (:then)
    (:else
      (if (Variables|/Game/ArcheryGame/Blueprints/Objetcs/BP_Arrow.BP_Arrow_C|GetisArrowGrabbed _asbp_arrow)
        (Utilities|FlowControl|Sequence
          (:then_0
            (bind _output_get (Variables|Default|SetAs%20BP%20Arrow _asbp_arrow))
            (Default|CallOnComponentReleased (Variables|/Game/ArcheryGame/Blueprints/Parents/BP_Grabbable.BP_Grabbable_C|GetBP_GrabComponent _output_get))
            (Default|TryRelease (Variables|/Game/ArcheryGame/Blueprints/Parents/BP_Grabbable.BP_Grabbable_C|GetBP_GrabComponent _output_get))
            (Variables|/Game/ArcheryGame/Blueprints/BP_GrabComponent.BP_GrabComponent_C|SetcanGrab (Variables|/Game/ArcheryGame/Blueprints/Parents/BP_Grabbable.BP_Grabbable_C|GetBP_GrabComponent _output_get) false)
            (Default|SetPrimitiveCompPhysics (Variables|/Game/ArcheryGame/Blueprints/Parents/BP_Grabbable.BP_Grabbable_C|GetBP_GrabComponent _output_get) false)
            (Transformation|SetActorLocationAndRotation (Variables|Default|GetAs%20BP%20Arrow) _locationvalue _rotatorvalue false true)
            (Transformation|AttachComponentToComponent (Variables|/Game/ArcheryGame/Blueprints/Parents/BP_Grabbable.BP_Grabbable_C|GetMesh (Variables|Default|GetAs%20BP%20Arrow)) (Variables|Character|GetMesh) "None" "KeepWorld" "KeepWorld" "KeepWorld" true))
          (:then_1
            (Variables|/Game/ArcheryGame/Blueprints/BP_GrabComponent.BP_GrabComponent_C|SetcanGrab (Variables|Default|GetBP_GrabComponent) true)
            (Variables|/Game/ArcheryGame/Blueprints/BP_GrabComponent.BP_GrabComponent_C|SetcanGrab (Variables|Default|GetBP_GrabComponentDraw) true)
            (Collision|SetCollisionResponsetoChannel (Variables|Default|GetSphere) "ECC_Visibility" "ECR_Block")))))))

(event OnDropped(BP_GrabComponentDraw)
  (bind _as_bp_arrow (Variables|Default|GetAs%20BP%20Arrow)
    (:then
      (Transformation|DetachFromComponent (Variables|/Game/ArcheryGame/Blueprints/Parents/BP_Grabbable.BP_Grabbable_C|GetMesh _as_bp_arrow) "KeepWorld" "KeepWorld" "KeepWorld" true)
      (bind _asbp_xrpawn (Utilities|Casting|CastToBP_XRPawn (Game|Player|GetPlayerPawn 0)))
      (Default|Shoot _asbp_xrpawn (Variables|Default|GetAs%20BP%20Arrow) (Math|Vector|GetForwardVector (Variables|Default|GetArrow2)))
      (Variables|Default|SetAs%20BP%20Arrow 0))
    (:else)))

(event EventBeginPlay)

(event Collision|EventActorBeginOverlap
  (params (OtherActor :type Actor%20Object%20Reference))
  (|CallParentFunction OtherActor) ; This node is disabled and will not be called.\nDrag off pins to build functionality.
)

(event EventTick
  (params (DeltaSeconds :type Float%20%28single-precision%29))
  (Rendering|Debug|DrawDebugSphere (Transformation|GetWorldLocation (Variables|Default|GetBP_GrabComponent)) 1e+01 12 "(R=1.000000,G=0.000000,B=0.608989,A=1.000000)" 0.0 2.0))

(fn ConstructionScript
  (|CallParentFunction))

(fn GetArrowLocation
  (bind _bp_grabcomponent (Variables|Default|GetBP_GrabComponent))
  (bind _is_right_hand (Variables|/Game/ArcheryGame/Blueprints/BP_GrabComponent.BP_GrabComponent_C|GetIs%20Right%20Hand _bp_grabcomponent))
  (return (select _is_right_hand (Transformation|GetWorldLocation (Variables|Default|GetRightHandedArrowSpot)) (Transformation|GetWorldLocation (Variables|Default|GetLeftHandedArrowSpot))) (select _is_right_hand (Transformation|GetWorldRotation (Variables|Default|GetRightHandedArrowSpot)) (Transformation|GetWorldRotation (Variables|Default|GetLeftHandedArrowSpot)))))