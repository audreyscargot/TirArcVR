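; BP_ArrowSpawner is an actor that supplies arrows for the XR archery game whenever a target round is prepared.
; On BeginPlay it binds to the BP_XRGameMode preparing-target event.
; When that fires, it spawns the arrow count from the game mode's difficulty data, scattering BP_Arrow actors randomly around its root and aligning them to the ArrowIndicator component's rotation.
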(event Custom|SpawningArrows
  (params (IntegerLevelDifficulty :type E_Difficulty%20Enum :default "NewEnumerator0"))
  (bind _as_bp_xrgame_mode (Variables|Default|GetAs%20BP%20XRGame%20Mode))
  (bind _difficultydata (Variables|/Game/XRFramework/Blueprints/BP_XRGameMode.BP_XRGameMode_C|GetDifficultyData _as_bp_xrgame_mode))
  (bind _arrowsquantity (Variables|/Game/ArcheryGame/Blueprints/DifficultyData/PDA_Difficulty.PDA_Difficulty_C|GetArrowsQuantity _difficultydata))
  (Development|PrintString (Utilities|String|ToString(Integer) _arrowsquantity))
  (for _index (range 0 (- _arrowsquantity 1))
    (Game|SpawnActorfromClass "/Game/ArcheryGame/Blueprints/Objetcs/BP_Arrow.BP_Arrow_C" (Math|Transform|MakeTransform (+ (Transformation|GetWorldLocation (Variables|Default|GetDefaultSceneRoot)) (Math|Vector|MakeVector (Math|Random|RandomFloatinRange -2e+01 2e+01) (Math|Random|RandomFloatinRange -2e+01 2e+01) 0.0)) (Transformation|GetWorldRotation (Variables|Default|GetArrowIndicator)) "1.000000,1.000000,1.000000") "AdjustIfPossibleButAlwaysSpawn" "MultiplyWithRoot" 0 0)))

(event EventBeginPlay
  (bind _asbp_xrgame_mode (Utilities|Casting|CastToBP_XRGameMode (Game|GetGameMode)))
  (bind _output_get (Variables|Default|SetAs%20BP%20XRGame%20Mode _asbp_xrgame_mode))
  (EventDispatchers|BindEventtoPreparingTarget _output_get (delegate Custom|SpawningArrows)))

(fn ConstructionScript)