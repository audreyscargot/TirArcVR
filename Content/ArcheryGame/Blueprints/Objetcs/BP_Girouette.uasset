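; Wind vane (girouette) actor for the archery game that sets and displays the wind for each level.
; On BeginPlay it binds to the XR game mode's preparing-target event, which passes difficulty and level.
; MakeWindref picks wind direction and strength from hardcoded per-level tables, ignoring difficulty.
; Its Arrow component hides at zero wind, rotates by a separate level table and stretches in X with wind magnitude.
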(event Custom|MakeWindref
  (params (IntegerLevelDifficulty :type E_Difficulty%20Enum :default "NewEnumerator0") (IntegerLevel :type Integer))
  (bind _arrow (Variables|Default|GetArrow))
  (Variables|Default|SetWindDirection (Utilities|Select :Index IntegerLevel :Option%200 "0, 0, 0" :Option%201 "0, 0, 0" :Option%202 "0.000000,-1.000000,0.000000" :Option%203 "0, 0, 0" :Option%204 "1.000000,1.000000,0.000000" :Option%205 "1.000000,0.000000,0.000000" :Option%206 "1.000000,-1.000000,0.000000" :Option%207 "-1.000000,-1.000000,0.000000" :Option%208 "-1.000000,0.000000,0.000000"))
  (Variables|Default|SetWindStrength (Utilities|Select :Index IntegerLevel :Option%200 0.0 :Option%201 0.0 :Option%202 0.2 :Option%203 0.0 :Option%204 0.2 :Option%205 0.2 :Option%206 0.2 :Option%207 0.2 :Option%208 0.2))
  (Development|SetHiddeninGame _arrow (Utilities|Operators|EqualEqual :A (Variables|Default|GetWindDirection)) false)
  (Transformation|SetRelativeRotation _arrow (Utilities|Select :Index IntegerLevel :Option%200 "0, 0, 0" :Option%201 "0, 0, 0" :Option%202 "0.000000,-90.000000,0.000000" :Option%203 "0.000000,0.000000,0.000000" :Option%204 "0.000000,45.000000,0.000000" :Option%205 "0.000000,90.000000,0.000000" :Option%206 "0.000000,-45.000000,0.000000" :Option%207 "0.000000,-135.000000,0.000000" :Option%208 "0.000000,-180.000000,0.000000") false false)
  (Transformation|SetRelativeScale3D _arrow (Math|Vector|MakeVector (* (Math|Vector|VectorLength (Variables|Default|GetWindDirection)) (Variables|Default|GetWindStrength) 1.5) 1.0 1.0)))

(event EventBeginPlay
  (bind _asbp_xrgame_mode (Utilities|Casting|CastToBP_XRGameMode (Game|GetGameMode)))
  (EventDispatchers|BindEventtoPreparingTarget _asbp_xrgame_mode (delegate Custom|MakeWindref)))

(fn ConstructionScript)