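; Archery target actor that awards points to the XR game mode based on where an arrow lands.
; It shows and enables collision only when the game mode's preparing-target event matches its difficulty.
; On a new arrow hit, it disables that arrow's collision, draws a debug sphere and indexes a score array by distance from the Sphere center in 10% radius bands.
; A MOVE event slides the cylinder along Y with a duration-scaled timeline.
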(event OnComponentHit(Cylinder)
  (params (HitComponent :type Primitive%20Component%20Object%20Reference) (OtherActor :type Actor%20Object%20Reference) (OtherComp :type Primitive%20Component%20Object%20Reference) (NormalImpulse :type Vector :default "0, 0, 0") (Hit :type Hit%20Result%20Structure%20%28by%20ref%29))
  (bind _impactpoint (Collision|BreakHitResult Hit))
  (bind _arrowscorearray (Variables|Default|GetArrowScoreArray))
  (bind _sphere (Variables|Default|GetSphere))
  (bind (_origin _boxextent _sphereradius) (Collision|GetComponentBounds _sphere))
  (bind _returnvalue (Math|Vector|Distance(Vector) _impactpoint _origin))
  (bind _returnvalue_2 (* _returnvalue 1e+02))
  (bind _returnvalue_3 (/ _returnvalue_2 _sphereradius))
  (bind _returnvalue_4 (/ _returnvalue_3 1e+01))
  (bind _returnvalue_5 (Math|Float|Floor _returnvalue_4))
  (bind _asbp_arrow (Utilities|Casting|CastToBP_Arrow OtherActor))
  (if (!= (Variables|Default|GetAs%20BP%20Arrow) _asbp_arrow)
    (bind _output_get (Variables|Default|SetAs%20BP%20Arrow _asbp_arrow))
    (Collision|SetActorEnableCollision _output_get false)
    (Rendering|Debug|DrawDebugSphere _impactpoint 7.0 12 "(R=0.000000,G=0.833595,B=1.000000,A=1.000000)" 1e+01 1.0)
    (if (Utilities|Array|IsValidIndex _arrowscorearray _returnvalue_5)
      (bind _output_get_2 (Variables|Default|SetArrowScore (Utilities|Array|Get(acopy) _arrowscorearray _returnvalue_5)))
      (Development|PrintString (Utilities|String|ToString(Integer) _output_get_2))
      (Default|AddScore (Variables|Default|GetAs%20BP%20XRGame%20Mode) _output_get_2))))

(event Custom|MakeDeactivate
  (params (IntegerLevelDifficulty :type E_Difficulty%20Enum :default "NewEnumerator0") (IntegerLevel :type Integer))
  (CallFunction|ActivateDeactivate (Utilities|Enum|Equal(Enum) IntegerLevelDifficulty (Variables|Default|GetTargetDifficulty))))

(event Custom|MOVE
  (Variables|Default|SetOGLoc (Transformation|GetActorLocation))
  (Components|Timeline|SetPlayRate (Variables|Default|GetTimeline) (/ 1.0 (Variables|Default|GetTimeforMove)))
  (bind _newtrack_0 (Timeline|Timeline Play)
    (:Update
      (Transformation|SetWorldLocation (Variables|Default|GetCylinder) (Math|Vector|MakeVector (.x (Variables|Default|GetOGLoc)) (Math|Float|Lerp (.y (Variables|Default|GetOGLoc)) (- (.y (Variables|Default|GetOGLoc)) 1e+02) _newtrack_0) (.z (Variables|Default|GetOGLoc))) true false))))

(event EventBeginPlay
  (bind _asbp_xrgame_mode (Utilities|Casting|CastToBP_XRGameMode (Game|GetGameMode)))
  (bind _output_get (Variables|Default|SetAs%20BP%20XRGame%20Mode _asbp_xrgame_mode))
  (EventDispatchers|BindEventtoPreparingTarget _output_get (delegate Custom|MakeDeactivate)))

(fn ConstructionScript)

(fn ActivateDeactivate
  (params (shouldActivate :type Boolean))
  (Rendering|SetVisibility (Variables|Default|GetCylinder) shouldActivate false)
  (Collision|SetActorEnableCollision shouldActivate)
  (Variables|Default|SetisActive shouldActivate))