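; BP_hiddenTarget is an archery target that awards points when a BP_Arrow hits it.
; On BeginPlay it binds to the XR game mode's target-preparation event, matching the difficulty against its own to set IsActive.
; That handler always shows the mesh and enables collision, whether or not the difficulty matches.
; An arrow hit disables collision, plays a sound, attaches the arrow and adds score through the game mode.
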(event OnComponentHit(target1v21)
  (params (HitComponent :type Primitive%20Component%20Object%20Reference) (OtherActor :type Actor%20Object%20Reference) (OtherComp :type Primitive%20Component%20Object%20Reference) (NormalImpulse :type Vector :default "0, 0, 0") (Hit :type Hit%20Result%20Structure%20%28by%20ref%29))
  (bind _asbp_arrow (Utilities|Casting|CastToBP_Arrow OtherActor))
  (Collision|SetActorEnableCollision false)
  (Audio|PlaySound2D "/Game/SoundDesign/ARC/Hit/SC_Hit.SC_Hit" 1.0 1.0 0.0 0 0)
  (Transformation|AttachActorToActor _asbp_arrow 0 "None" "KeepWorld" "KeepWorld" "KeepWorld" true)
  (Default|AddScore (Variables|Default|GetAs%20BP%20XRGame%20Mode) (Variables|Default|GetPointOfTarget)))

(event Custom|MakeDeactivate
  (params (IntegerLevelDifficulty :type E_Difficulty%20Enum :default "NewEnumerator0") (IntegerLevel :type Integer))
  (CallFunction|ActivateDeactivate (Utilities|Enum|Equal(Enum) IntegerLevelDifficulty (Variables|Default|GetTargetDifficulty))))

(event EventBeginPlay
  (bind _asbp_xrgame_mode (Utilities|Casting|CastToBP_XRGameMode (Game|GetGameMode)))
  (bind _output_get (Variables|Default|SetAs%20BP%20XRGame%20Mode _asbp_xrgame_mode))
  (EventDispatchers|BindEventtoPreparingTarget _output_get (delegate Custom|MakeDeactivate)))

(event Collision|EventActorBeginOverlap
  (params (OtherActor :type Actor%20Object%20Reference)))

(event EventTick
  (params (DeltaSeconds :type Float%20%28single-precision%29)))

(fn ConstructionScript)

(fn ActivateDeactivate
  (params (shouldActivate :type Boolean))
  (Rendering|SetVisibility (Variables|Default|Gettarget1v21) true false)
  (Collision|SetActorEnableCollision true)
  (Variables|Default|SetisActive shouldActivate))