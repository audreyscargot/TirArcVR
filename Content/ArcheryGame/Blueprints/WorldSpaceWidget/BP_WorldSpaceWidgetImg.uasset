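; BP_WorldSpaceWidgetImg is an actor that shows an image widget in world space in the archery XR game.
; On BeginPlay it binds an event to the SpawnWidgetIMG dispatcher of BP_XRGameMode.
; Its spawnWidget event selects by WidgetType, creating WBP_ArrowRedif for the Arrow Redif case and assigning it to the Widget component.
; The afficher and remove events show and hide that component.
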(event Custom|spawnWidget
  (switch Utilities|FlowControl|Switch|SwitchonE_Widget (Variables|Default|GetwidgetType)
    (:NewEnumerator6
      (bind _returnvalue (UserInterface|CreateWidget "/Game/ArcheryGame/Widgets/WBP_ArrowRedif.WBP_ArrowRedif_C"))
      (UserInterface|SetWidget (Variables|Default|GetWidget) _returnvalue))))

(event Custom|afficher
  (Development|SetHiddeninGame (Variables|Default|GetWidget) false false))

(event Custom|remove
  (Development|SetHiddeninGame (Variables|Default|GetWidget) true false))

(event EventBeginPlay
  (bind _asbp_xrgame_mode (Utilities|Casting|CastToBP_XRGameMode (Game|GetGameMode)))
  (EventDispatchers|BindEventtoSpawnWidgetIMG _asbp_xrgame_mode (EventDispatchers|CreateEvent :!event Custom|spawnWidget)))

(fn ConstructionScript)