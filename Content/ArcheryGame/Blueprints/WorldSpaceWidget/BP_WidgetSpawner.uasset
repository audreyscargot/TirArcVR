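; BP_WidgetSpawner is an actor that spawns a world-space UI widget at its own transform in the archery game.
; Its Spawn event creates a BP_WorldSpaceWidget with the given widget type and keeps a reference to it.
; On BeginPlay it binds to the XR game mode's PreparingTarget event, which destroys the spawned widget if it is still valid.
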(event Custom|Spawn
  (params (WidgetType :type E_Widget%20Enum :default "NewEnumerator0"))
  (bind _returnvalue (Game|SpawnActorfromClass "/Game/ArcheryGame/Blueprints/WorldSpaceWidget/BP_WorldSpaceWidget.BP_WorldSpaceWidget_C" (Transformation|GetActorTransform) "Undefined" "MultiplyWithRoot" 0 WidgetType 0))
  (Variables|Default|SetWidgetRef _returnvalue))

(event Custom|Destroy
  (params (IntegerLevelDifficulty :type E_Difficulty%20Enum :default "NewEnumerator0") (IntegerLevel :type Integer))
  (bind _widgetref (Variables|Default|GetWidgetRef))
  (Utilities|IsValid _widgetref
    (:Is%20Valid
      (Actor|DestroyActor _widgetref))))

(event EventBeginPlay
  (bind _asbp_xrgame_mode (Utilities|Casting|CastToBP_XRGameMode (Game|GetGameMode)))
  (EventDispatchers|BindEventtoPreparingTarget _asbp_xrgame_mode (delegate Custom|Destroy)))

(fn ConstructionScript)